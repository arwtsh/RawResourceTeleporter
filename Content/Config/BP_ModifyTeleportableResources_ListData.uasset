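; List data object for one resource entry in the Modify Teleportable Resources config list, wrapping an item descriptor class.
; Setting the descriptor caches its item name, while the small icon is read from the descriptor on request.
; Selection state is not stored locally: it reads, adds or removes the descriptor in the Parent's selected resources collection and logs each change.
; The selection-changed callback is left unwired.
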(fn `GetDescriptor`
  (returns (return :type "FGItemDescriptor Class Reference"))
  (return (`self.descriptor`)))

(fn `GetIcon`
  (returns (NewParam :type "Texture2D Object Reference"))
  (bind _descriptor (`self.descriptor`))
  (return (select `bool` (`KismetSystemLibrary.IsValidClass` _descriptor) :`true` (`FGItemDescriptor.GetSmallIcon` _descriptor))))

(fn `GetIsSelected`
  (returns (ReturnValue :type Boolean))
  (bind _selectedresources (`/RawResourceTeleporter/Config/Widget_ModifyTeleportableResources.GetSelectedResources` (`self.parent`)))
  (return (`BlueprintSetLibrary.Set_Contains` _selectedresources (`self.descriptor`))))

(fn `GetItemName`
  (returns (DisplayName :type Text))
  (return (`self.name`)))

(fn `SetDescriptor`
  (params (descriptor :type "FGItemDescriptor Class Reference"))
  (bind _output_get (set `self.descriptor` descriptor))
  (`self.SetItemName` (`FGItemDescriptor.GetItemName` _output_get)))

(fn `SetIsSelected`
  (params (IsSelected :type Boolean))
  (bind _descriptor (`self.descriptor`))
  (bind _selectedresources (`/RawResourceTeleporter/Config/Widget_ModifyTeleportableResources.GetSelectedResources` (`self.parent`)))
  (if IsSelected
    (`BlueprintSetLibrary.Set_Add` _selectedresources _descriptor)
    (`BlueprintLoggingLibrary.LogDisplay` "Add item")
    (else
      (`BlueprintSetLibrary.Set_Remove` _selectedresources _descriptor)
      (`BlueprintLoggingLibrary.LogDisplay` "Remove item")))
  (`BlueprintLoggingLibrary.LogDisplay` (`KismetStringLibrary.Conv_IntToString` (`BlueprintSetLibrary.Set_Length` _selectedresources))))

(fn `SetItemName`
  (params (name :type Text))
  (set `self.name` name))